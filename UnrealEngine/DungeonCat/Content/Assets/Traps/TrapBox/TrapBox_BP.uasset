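; Trap control box that a character reveals and uses to disable its linked spike, arrow and spin traps.
; It starts with grey materials and a hidden lever, and outlines on overlap until used.
; The thief trigger freezes movement, restores materials, animates door and lever by timelines, then deactivates ControlledTraps and re-enables movement after a delay.
; Tick also computes a thief-distance visibility value, unused here; the Thief lookup is disconnected.
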(event `self.ReceiveBeginPlay`
  (bind _trapbox_main (`self.TrapBox_Main`))
  (bind _trapbox_door (`self.TrapBox_Door`))
  ;[1 1 1] Set Transp Mat
  (set `self.OrgMaterials_Main` (`MeshComponent.GetMaterials` (`self.TrapBox_Main`)))
  (set `self.OrgMaterials_Door` (`MeshComponent.GetMaterials` (`self.TrapBox_Door`)))
  (`|ExecutionSequence`
    (:`then_0`
      (`PrimitiveComponent.SetMaterial` _trapbox_main 0 "/Game/Assets/WorldMaterials/TrapMaterials/Trap_Grey_02.Trap_Grey_02")
      (`PrimitiveComponent.SetMaterial` _trapbox_main 1 "/Game/Assets/WorldMaterials/TrapMaterials/Trap_Grey.Trap_Grey")
      (`PrimitiveComponent.SetMaterial` _trapbox_main 2 "/Game/Assets/WorldMaterials/TrapMaterials/Trap_Grey.Trap_Grey"))
    (:`then_1`
      (`PrimitiveComponent.SetMaterial` _trapbox_door 0 "/Game/Assets/WorldMaterials/TrapMaterials/Trap_Grey.Trap_Grey")
      (`PrimitiveComponent.SetMaterial` _trapbox_door 1 "/Game/Assets/WorldMaterials/TrapMaterials/Trap_Grey_02.Trap_Grey_02"))
    (:`then_2`
      (`SceneComponent.SetVisibility` (`self.TrapBox_Lever`) false false))))

(event `EventTick #2`
  ;[1 1 1] SET TRANSP MAT - Sjukt Ooptimerat, fixa
  (if (not (`self.IsFound?`))
    (`|ExecutionSequence`
      (:`then_0`
        (if (`self.IsActiveThief?`)
          (set `self.Visbility` (`KismetMathLibrary.FClamp` (- (+ (* (`KismetMathLibrary.MapRangeClamped` (/ (`KismetMathLibrary.VSize` (- (`self.K2_GetActorLocation` (`self.Thief`)) (`self.K2_GetActorLocation` self))) 10.0) 10.0 100.0 0.0 1.0) -1.0) 1.0) (`self.VisbilityMinus`)))))))))

(event `self.ReceiveTick`
  (params (DeltaSeconds :type "Float (single-precision)"))
  (`self.EventTick #2`)
  (bind _astop_down_character (cast `/Game/Blueprints/TopDownCharacter` (`self.TempActor`)))
  (if (`/Game/Blueprints/TopDownCharacter.RTriggerThief_Pressed` _astop_down_character)
    (bind _charactermovement (`Character.CharacterMovement` _astop_down_character))
    (`MovementComponent.StopMovementImmediately` _charactermovement)
    (set `self.IsFound?` true)
    (`ActorComponent.SetActive` _charactermovement false false)
    (`|ExecutionSequence`
      (:`then_0`
        ;[1 1 1] Open Door and Pull Down Lever
        (`/Engine/EditorBlueprintResources/StandardMacros.DoOnce` false
          (:`Completed`
            (`PrimitiveComponent.SetRenderCustomDepth` (`self.DummyOutlineMesh`) false)
            (bind (_direction _newtrack_0) (`Timeline|Timeline_0` :!via `PlayFromStart`)
              (:`Update`
                (`SceneComponent.K2_SetRelativeRotation` (`self.TrapBox_Door`) (`KismetMathLibrary.RLerp` (struct) (struct :`Yaw` -160.0) _newtrack_0) false false))
              (:`Finished`
                (`KismetSystemLibrary.Delay` 1.0)
                (bind (_direction_2 _newtrack_0_2) (`Timeline|Timeline_1` :!via `PlayFromStart`)
                  (:`Update`
                    (`SceneComponent.K2_SetRelativeLocation` (`self.TrapBox_Lever`) (`KismetMathLibrary.VLerp` (0.0 0.0 0.0) (0.0 0.0 -12.0) _newtrack_0_2) false false)
                    (set `self.IsUsed?` true))))))))
      (:`then_1`
        ;[1 1 1] Disable These types of BPs
        (`KismetSystemLibrary.Delay` 2.0)
        (for _array_element (`self.ControlledTraps`)
          (`|ExecutionSequence`
            (:`then_0`
              (bind _asfloor_spike_trap_bp (cast `/Game/Assets/Traps/FloorSpikeTrap/FloorSpikeTrap_BP` _array_element))
              (set `/Game/Assets/Traps/FloorSpikeTrap/FloorSpikeTrap_BP.IsActive?` false _asfloor_spike_trap_bp))
            (:`then_1`
              (bind _asarrow_trap_bp (cast `/Game/Assets/Traps/ArrowTrap/ArrowTrap_BP` _array_element))
              (set `/Game/Assets/Traps/ArrowTrap/ArrowTrap_BP.IsActive?` false _asarrow_trap_bp))
            (:`then_2`
              (bind _asspin_trap_double_wall_midsize_bp (cast `/Game/Assets/Traps/SpinTrap/SpinTrap_DoubleWall_Midsize_BP` _array_element))
              (set `/Game/Assets/Traps/SpinTrap/SpinTrap_DoubleWall_Midsize_BP.IsActive?` false _asspin_trap_double_wall_midsize_bp))
            (:`then_3`
              (bind _asspin_trap_no_wall_long_bp (cast `/Game/Assets/Traps/SpinTrap/SpinTrap_NoWall_Long_BP` _array_element))
              (set `/Game/Assets/Traps/SpinTrap/SpinTrap_NoWall_Long_BP.IsActive?` false _asspin_trap_no_wall_long_bp))))
        ;[1 1 1] Enable Actor Movement again
        (`ActorComponent.SetActive` _charactermovement true false))
      (:`then_2`
        (`/Engine/EditorBlueprintResources/StandardMacros.DoOnce` false
          (:`Completed`
            (set `self.IsFound?` true)
            (`|ExecutionSequence`
              (:`then_0`
                (for (_array_element_2 _array_index) (`self.OrgMaterials_Main`)
                  (`PrimitiveComponent.SetMaterial` (`self.TrapBox_Main`) _array_index _array_element_2)))
              (:`then_1`
                (`SceneComponent.SetVisibility` (`self.TrapBox_Lever`) true false))
              (:`then_2`
                (for (_array_element_3 _array_index_2) (`self.OrgMaterials_Door`)
                  (`PrimitiveComponent.SetMaterial` (`self.TrapBox_Door`) _array_index_2 _array_element_3))))))))))

(event `self.ReceiveActorBeginOverlap`
  (params (OtherActor :type "Actor Object Reference"))
  (set `self.TempActor` OtherActor)
  (if (not (`self.IsUsed?`))
    (`PrimitiveComponent.SetRenderCustomDepth` (`self.DummyOutlineMesh`) true)))

(event `self.ReceiveActorEndOverlap`
  (params (OtherActor :type "Actor Object Reference"))
  (set `self.TempActor` null)
  (`PrimitiveComponent.SetRenderCustomDepth` (`self.DummyOutlineMesh`) false))

(fn `BeginOutlineFocus`
  (returns (Success :type Boolean))
  (return false))

(fn `EndOutlineFocus`
  (returns (Success :type Boolean))
  (return false))

(fn `GetIsActorUsable`
  (returns (IsUsable :type Boolean))
  (return false))

(fn `GetUseActionText`
  (returns (ActionText :type Text))
  (return ""))

(fn `OnActorUsed`
  (params (Controller :type "PlayerController Object Reference"))
  (returns (Success :type Boolean))
  (return false))

(fn `UserConstructionScript`)