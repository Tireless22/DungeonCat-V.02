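; Floor spike trap that disguises itself with swapped tile materials and springs when a TopDownCharacter steps on it.
; Overlap triggers delayed timelines that raise and retract four spikes; hits only print, as a damage placeholder.
; While active and unfound, Tick searches for the Thief each frame and computes a distance-based visibility value, without applying it here.
; The original floor materials return once the trap has fired or is inactive.
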(event `self.ReceiveTick`
  (params (DeltaSeconds :type "Float (single-precision)"))
  ;[1 1 1] SET TRANSP MAT - Sjukt Ooptimerat, fixa
  (if (`self.IsActive?`)
    (if (not (`self.IsFound?`))
      (`|ExecutionSequence`
        (:`then_0`
          (set `self.Visbility` (`KismetMathLibrary.FClamp` (- (+ (* (`KismetMathLibrary.MapRangeClamped` (/ (`KismetMathLibrary.VSize` (- (`self.K2_GetActorLocation` (`self.Thief`)) (`self.K2_GetActorLocation` self))) 10.0) 10.0 100.0 0.0 1.0) -1.0) 1.0) (`self.Visibility Minus`)))))
        (:`then_1`
          (bind _outactors (`GameplayStatics.GetAllActorsOfClass` "/Game/Blueprints/Blueprints/TopDownCharacter.TopDownCharacter_C"))
          (for _array_element _outactors
            (if (`|EnumEquality` (`/Game/Blueprints/Blueprints/TopDownCharacter.IsClass` _array_element) "NewEnumerator2")
              (set `self.Thief` _array_element))))))
    (else
      (`/Engine/EditorBlueprintResources/StandardMacros.DoOnce` false
        (:`Completed`
          (for (_array_element_2 _array_index) (`self.OrgMaterials`)
            (`PrimitiveComponent.SetMaterial` (`self.FloorTile`) _array_index _array_element_2)))))))

(event `self.ReceiveBeginPlay`
  (bind _floortile (`self.FloorTile`))
  ;[1 1 1] Set Transp Mat
  (set `self.OrgMaterials` (`MeshComponent.GetMaterials` (`self.FloorTile`)))
  (`PrimitiveComponent.SetMaterial` _floortile 0 "/Game/Assets/WorldMaterials/TrapMaterials/Trap_Brown.Trap_Brown")
  (`PrimitiveComponent.SetMaterial` _floortile 1 "/Game/Assets/WorldMaterials/TrapMaterials/Trap_Grey.Trap_Grey")
  (`PrimitiveComponent.SetMaterial` _floortile 2 "/Game/Assets/WorldMaterials/TrapMaterials/Trap_Black.Trap_Black"))

(event `self.TrapDetection.OnComponentBeginOverlap`
  (params (OtherActor :type "Actor Object Reference") (OtherComp :type "PrimitiveComponent Object Reference") (OtherBodyIndex :type Integer) (bFromSweep :type Boolean) (SweepResult :type "HitResult Structure (by ref)"))
  (bind _spike_01 (`self.Spike_01`))
  (cast `/Game/Blueprints/Blueprints/TopDownCharacter` OtherActor)
  (if (and (not (`self.IsAtPeak?`)) (`self.IsActive?`))
    (`KismetSystemLibrary.Delay` 0.3)
    (bind (_direction _newtrack_0) (`Timeline|Timeline_0` :!via `PlayFromStart`)
      (:`Update`
        (`SceneComponent.K2_SetRelativeLocation` _spike_01 (`KismetMathLibrary.VLerp` (0.0 0.0 -60.0) (0.0 0.0 0.0) _newtrack_0) false false)
        (`SceneComponent.K2_SetRelativeLocation` (`self.Spike_02`) (`KismetMathLibrary.VLerp` (0.0 0.0 -60.0) (0.0 0.0 0.0) _newtrack_0) false false)
        (`SceneComponent.K2_SetRelativeLocation` (`self.Spike_03`) (`KismetMathLibrary.VLerp` (0.0 0.0 -60.0) (0.0 0.0 0.0) _newtrack_0) false false)
        (`SceneComponent.K2_SetRelativeLocation` (`self.Spike_04`) (`KismetMathLibrary.VLerp` (0.0 0.0 -60.0) (0.0 0.0 0.0) _newtrack_0) false false))
      (:`Finished`
        (set `self.IsAtPeak?` true)
        (`|ExecutionSequence`
          (:`then_0`
            (`KismetSystemLibrary.Delay` 2.0)
            (bind (_direction_2 _newtrack_0_2) (`Timeline|Timeline_1` :!via `PlayFromStart`)
              (:`Update`
                (`SceneComponent.K2_SetRelativeLocation` _spike_01 (`KismetMathLibrary.VLerp` (0.0 0.0 0.0) (0.0 0.0 -60.0) _newtrack_0_2) false false)
                (`SceneComponent.K2_SetRelativeLocation` (`self.Spike_02`) (`KismetMathLibrary.VLerp` (0.0 0.0 0.0) (0.0 0.0 -60.0) _newtrack_0_2) false false)
                (`SceneComponent.K2_SetRelativeLocation` (`self.Spike_03`) (`KismetMathLibrary.VLerp` (0.0 0.0 0.0) (0.0 0.0 -60.0) _newtrack_0_2) false false)
                (`SceneComponent.K2_SetRelativeLocation` (`self.Spike_04`) (`KismetMathLibrary.VLerp` (0.0 0.0 0.0) (0.0 0.0 -60.0) _newtrack_0_2) false false))
              (:`Finished`
                (set `self.IsAtPeak?` false))))
          (:`then_1`
            (`/Engine/EditorBlueprintResources/StandardMacros.DoOnce` false
              (:`Completed`
                (set `self.IsFound?` true)
                (for (_array_element _array_index) (`self.OrgMaterials`)
                  (`PrimitiveComponent.SetMaterial` (`self.FloorTile`) _array_index _array_element))))))))))

(event `self.Spike_04.OnComponentBeginOverlap`
  (params (OtherActor :type "Actor Object Reference") (OtherComp :type "PrimitiveComponent Object Reference") (OtherBodyIndex :type Integer) (bFromSweep :type Boolean) (SweepResult :type "HitResult Structure (by ref)"))
  (cast `/Game/Blueprints/Blueprints/TopDownCharacter` OtherActor)
  (if (not (`self.IsAtPeak?`)) :!label _label
    ;[1 1 1] Add Damage Code Here
    (`KismetSystemLibrary.PrintString` "HIT" true true (struct :`R` 1.0 :`G` 0.057093 :`A` 1.0) 1.0)))

(event `self.Spike_02.OnComponentBeginOverlap`
  (params (OtherActor :type "Actor Object Reference") (OtherComp :type "PrimitiveComponent Object Reference") (OtherBodyIndex :type Integer) (bFromSweep :type Boolean) (SweepResult :type "HitResult Structure (by ref)"))
  (cast `/Game/Blueprints/Blueprints/TopDownCharacter` OtherActor)
  (goto _label))

(event `self.Spike_03.OnComponentBeginOverlap`
  (params (OtherActor :type "Actor Object Reference") (OtherComp :type "PrimitiveComponent Object Reference") (OtherBodyIndex :type Integer) (bFromSweep :type Boolean) (SweepResult :type "HitResult Structure (by ref)"))
  (cast `/Game/Blueprints/Blueprints/TopDownCharacter` OtherActor)
  (goto _label))

(event `self.Spike_01.OnComponentBeginOverlap`
  (params (OtherActor :type "Actor Object Reference") (OtherComp :type "PrimitiveComponent Object Reference") (OtherBodyIndex :type Integer) (bFromSweep :type Boolean) (SweepResult :type "HitResult Structure (by ref)"))
  (cast `/Game/Blueprints/Blueprints/TopDownCharacter` OtherActor)
  (goto _label))

(fn `UserConstructionScript`)