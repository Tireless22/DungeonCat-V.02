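; Long, wall-less spin trap whose blade rises, spins while sliding along a track, then sinks, alternating direction each pass.
; Tick starts passes while IsActive is set and a TopDownCharacter is inside the Detection volume.
; Chained timelines lerp the blade's relative location and rotation, with DoOnce gates and a SecondTime flag sequencing the two directions.
; Blade hits on the character only print a debug message, applying no damage.
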(event `self.ReceiveTick`
  (params (DeltaSeconds :type "Float (single-precision)"))
  (bind _spinblade (`self.SpinBlade`))
  (bind _spinblade_2 (`self.SpinBlade`))
  (if (`self.IsActive?`)
    (if (`self.PlayerInRange?`)
      (if (`self.SecondTime?`)
        (`/Engine/EditorBlueprintResources/StandardMacros.DoOnce` false :!label _label
          (:`Completed`
            (bind (_direction _newtrack_0) (`Timeline|Timeline_4` :!via `PlayFromStart`)
              (:`Update`
                (`SceneComponent.K2_SetRelativeLocation` (`self.SpinBlade`) (`KismetMathLibrary.VLerp` (300.0 0.0 -55.0) (300.0 0.0 10.0) _newtrack_0) false false))
              (:`Finished`
                (bind (_direction_2 _newtrack_0_2) (`Timeline|Timeline_1` :!via `PlayFromStart`)
                  (:`Update`
                    (`|ExecutionSequence`
                      (:`then_0`
                        (`SceneComponent.K2_SetRelativeRotation` _spinblade (`KismetMathLibrary.RLerp` (struct) (struct :`Pitch` -720.0) _newtrack_0_2) false false))
                      (:`then_1`
                        (`SceneComponent.K2_SetRelativeLocation` _spinblade (`KismetMathLibrary.VLerp` (300.0 0.0 10.0) (-175.0 0.0 10.0) _newtrack_0_2) false false))))
                  (:`Finished`
                    (bind (_direction_3 _newtrack_0_3) (`Timeline|Timeline_5` :!via `PlayFromStart`)
                      (:`Update`
                        (`SceneComponent.K2_SetRelativeLocation` (`self.SpinBlade`) (`KismetMathLibrary.VLerp` (-175.0 0.0 10.0) (-175.0 0.0 -55.0) _newtrack_0_3) false false))
                      (:`Finished`
                        (set `self.SecondTime?` false)
                        (goto _label_2 :!via `Reset`)))))))))
        (else
          (`/Engine/EditorBlueprintResources/StandardMacros.DoOnce` false :!label _label_2
            (:`Completed`
              (bind (_direction_4 _newtrack_0_4) (`Timeline|Timeline_2` :!via `PlayFromStart`)
                (:`Update`
                  (`SceneComponent.K2_SetRelativeLocation` (`self.SpinBlade`) (`KismetMathLibrary.VLerp` (-175.0 0.0 -55.0) (-175.0 0.0 10.0) _newtrack_0_4) false false))
                (:`Finished`
                  (bind (_direction_5 _newtrack_0_5) (`Timeline|Timeline_0` :!via `PlayFromStart`)
                    (:`Update`
                      (`|ExecutionSequence`
                        (:`then_0`
                          (`SceneComponent.K2_SetRelativeRotation` _spinblade_2 (`KismetMathLibrary.RLerp` (struct) (struct :`Pitch` -720.0) _newtrack_0_5) false false))
                        (:`then_1`
                          (`SceneComponent.K2_SetRelativeLocation` _spinblade_2 (`KismetMathLibrary.VLerp` (-175.0 0.0 10.0) (300.0 0.0 10.0) _newtrack_0_5) false false))))
                    (:`Finished`
                      (bind (_direction_6 _newtrack_0_6) (`Timeline|Timeline_3` :!via `PlayFromStart`)
                        (:`Update`
                          (`SceneComponent.K2_SetRelativeLocation` (`self.SpinBlade`) (`KismetMathLibrary.VLerp` (300.0 0.0 10.0) (300.0 0.0 -55.0) _newtrack_0_6) false false))
                        (:`Finished`
                          (set `self.SecondTime?` true)
                          (goto _label :!via `Reset`))))))))))))))

(event `self.Detection.OnComponentBeginOverlap`
  (params (OtherActor :type "Actor Object Reference") (OtherComp :type "PrimitiveComponent Object Reference") (OtherBodyIndex :type Integer) (bFromSweep :type Boolean) (SweepResult :type "HitResult Structure (by ref)"))
  (cast `/Game/Blueprints/Blueprints/TopDownCharacter` OtherActor)
  (set `self.PlayerInRange?` true))

(event `self.Detection.OnComponentEndOverlap`
  (params (OtherActor :type "Actor Object Reference") (OtherComp :type "PrimitiveComponent Object Reference") (OtherBodyIndex :type Integer))
  (cast `/Game/Blueprints/Blueprints/TopDownCharacter` OtherActor)
  (set `self.PlayerInRange?` false))

(event `self.SpinBlade.OnComponentHit`
  (params (OtherActor :type "Actor Object Reference") (OtherComp :type "PrimitiveComponent Object Reference") (NormalImpulse :type "Vector Structure") (Hit :type "HitResult Structure (by ref)"))
  (cast `/Game/Blueprints/Blueprints/TopDownCharacter` OtherActor)
  (`KismetSystemLibrary.PrintString` "HIT!" true true (struct :`R` 1.0 :`G` 0.029568 :`A` 1.0)))

(fn `UserConstructionScript`)