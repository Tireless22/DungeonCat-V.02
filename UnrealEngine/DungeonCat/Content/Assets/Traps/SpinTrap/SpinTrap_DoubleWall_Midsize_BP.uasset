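; Mid-size double-wall spin trap whose blade spins and slides between two end points while active and a TopDownCharacter is inside its Detection volume.
; Two timelines alternate the stroke direction through cross-resetting DoOnce gates.
; BeginPlay caches wall materials and applies substitutes, restored once when the trap is triggered or inactive.
; Until found, Tick can compute a thief-distance visibility value, not applied here; blade hits only print "HIT!".
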(event `self.ReceiveBeginPlay`
  (bind _wallend2 (`self.WallEnd2`))
  ;[1 1 1] Set Transp Mat
  (set `self.OrgMaterials_main` (`MeshComponent.GetMaterials` (`self.Main`)))
  (set `self.OrgMaterials_WallEnd` (`MeshComponent.GetMaterials` (`self.WallEnd`)))
  (`|ExecutionSequence`
    (:`then_0`
      (`PrimitiveComponent.SetMaterial` (`self.Main`) 0 "/Game/Assets/WorldMaterials/TrapMaterials/Trap_Grey_02.Trap_Grey_02")
      (`PrimitiveComponent.SetMaterial` (`self.mainCont`) 0 "/Game/Assets/WorldMaterials/TrapMaterials/Trap_Grey_02.Trap_Grey_02")
      (`PrimitiveComponent.SetMaterial` (`self.mainCont`) 1 "/Game/Assets/WorldMaterials/TrapMaterials/Trap_Black.Trap_Black")
      (`PrimitiveComponent.SetMaterial` (`self.Main`) 1 "/Game/Assets/WorldMaterials/TrapMaterials/Trap_Black.Trap_Black"))
    (:`then_1`
      (`PrimitiveComponent.SetMaterial` _wallend2 0 "/Game/Assets/WorldMaterials/TrapMaterials/Trap_Black.Trap_Black")
      (`PrimitiveComponent.SetMaterial` (`self.WallEnd`) 0 "/Game/Assets/WorldMaterials/TrapMaterials/Trap_Black.Trap_Black")
      (`PrimitiveComponent.SetMaterial` (`self.WallEnd`) 1 "/Game/Assets/WorldMaterials/TrapMaterials/Trap_Grey_02.Trap_Grey_02")
      (`PrimitiveComponent.SetMaterial` _wallend2 1 "/Game/Assets/WorldMaterials/TrapMaterials/Trap_Grey_02.Trap_Grey_02")
      (`PrimitiveComponent.SetMaterial` _wallend2 2 "/Game/Assets/WorldMaterials/TrapMaterials/Trap_Black.Trap_Black")
      (`PrimitiveComponent.SetMaterial` (`self.WallEnd`) 2 "/Game/Assets/WorldMaterials/TrapMaterials/Trap_Black.Trap_Black"))))

(event `Event Tick #2`
  ;[1 1 1] SET TRANSP MAT - Sjukt Ooptimerat, fixa
  (if (`self.IsActive?`)
    (if (not (`self.IsFound?`))
      (if (`self.IsActiveThief?`)
        (set `self.Visbility` (`KismetMathLibrary.FClamp` (- (+ (* (`KismetMathLibrary.MapRangeClamped` (/ (`KismetMathLibrary.VSize` (- (`self.K2_GetActorLocation` (`self.Thief`)) (`self.K2_GetActorLocation` self))) 10.0) 10.0 100.0 0.0 1.0) -1.0) 1.0) (`self.VisbilityMinus`))))))
    (else
      (`/Engine/EditorBlueprintResources/StandardMacros.DoOnce` false
        (:`Completed`
          (`self.Reset Materials`))))))

(event `self.ReceiveTick`
  (params (DeltaSeconds :type "Float (single-precision)"))
  (bind _spinblade (`self.SpinBlade`))
  (bind _spinblade_2 (`self.SpinBlade`))
  (`self.Event Tick #2`)
  (if (`self.IsActive?`)
    (if (`self.PlayerInRange?`)
      (set `self.IsFound?` true)
      (`|ExecutionSequence`
        (:`then_0`
          (if (`self.SecondTime?`)
            ;[1 1 1] Move Blade from Point A to Point B
            (`/Engine/EditorBlueprintResources/StandardMacros.DoOnce` false :!label _label
              (:`Completed`
                (bind (_direction _newtrack_0) (`Timeline|Timeline_1` :!via `PlayFromStart`)
                  (:`Update`
                    (`|ExecutionSequence`
                      (:`then_0`
                        (`SceneComponent.K2_SetRelativeRotation` _spinblade (`KismetMathLibrary.RLerp` (struct) (struct :`Pitch` -720.0) _newtrack_0) false false))
                      (:`then_1`
                        (`SceneComponent.K2_SetRelativeLocation` _spinblade (`KismetMathLibrary.VLerp` (300.0 0.0 10.0) (-240.0 0.0 10.0) _newtrack_0) false false))))
                  (:`Finished`
                    (set `self.SecondTime?` false)
                    (goto _label_2 :!via `Reset`)))))
            (else
              (`/Engine/EditorBlueprintResources/StandardMacros.DoOnce` false :!label _label_2
                (:`Completed`
                  (bind (_direction_2 _newtrack_0_2) (`Timeline|Timeline_0` :!via `PlayFromStart`)
                    (:`Update`
                      (`|ExecutionSequence`
                        (:`then_0`
                          (`SceneComponent.K2_SetRelativeRotation` _spinblade_2 (`KismetMathLibrary.RLerp` (struct) (struct :`Pitch` -720.0) _newtrack_0_2) false false))
                        (:`then_1`
                          (`SceneComponent.K2_SetRelativeLocation` _spinblade_2 (`KismetMathLibrary.VLerp` (-240.0 0.0 10.0) (300.0 0.0 10.0) _newtrack_0_2) false false))))
                    (:`Finished`
                      (set `self.SecondTime?` true)
                      (goto _label :!via `Reset`))))))))
        (:`then_1`
          (`/Engine/EditorBlueprintResources/StandardMacros.DoOnce` false
            (:`Completed`
              (`self.Reset Materials`))))))))

(event `self.Detection.OnComponentBeginOverlap`
  (params (OtherActor :type "Actor Object Reference") (OtherComp :type "PrimitiveComponent Object Reference") (OtherBodyIndex :type Integer) (bFromSweep :type Boolean) (SweepResult :type "HitResult Structure (by ref)"))
  (cast `/Game/Blueprints/TopDownCharacter` OtherActor)
  (set `self.PlayerInRange?` true))

(event `self.Detection.OnComponentEndOverlap`
  (params (OtherActor :type "Actor Object Reference") (OtherComp :type "PrimitiveComponent Object Reference") (OtherBodyIndex :type Integer))
  (cast `/Game/Blueprints/TopDownCharacter` OtherActor)
  (set `self.PlayerInRange?` false))

(event `self.SpinBlade.OnComponentHit`
  (params (OtherActor :type "Actor Object Reference") (OtherComp :type "PrimitiveComponent Object Reference") (NormalImpulse :type "Vector Structure") (Hit :type "HitResult Structure (by ref)"))
  ;[1 1 1] Hit Detection. Make better with DMG loss
  (cast `/Game/Blueprints/TopDownCharacter` OtherActor)
  (`KismetSystemLibrary.PrintString` "HIT!" true true (struct :`R` 1.0 :`G` 0.029568 :`A` 1.0)))

(fn `Reset Materials`
  (`|ExecutionSequence`
    (:`then_0`
      (for (_array_element _array_index) (`self.OrgMaterials_main`)
        (`PrimitiveComponent.SetMaterial` (`self.Main`) _array_index _array_element)
        (`PrimitiveComponent.SetMaterial` (`self.mainCont`) _array_index _array_element)))
    (:`then_1`
      (for (_array_element_2 _array_index_2) (`self.OrgMaterials_WallEnd`)
        (`PrimitiveComponent.SetMaterial` (`self.WallEnd2`) _array_index_2 _array_element_2)
        (`PrimitiveComponent.SetMaterial` (`self.WallEnd`) _array_index_2 _array_element_2)))))

(fn `UserConstructionScript`)