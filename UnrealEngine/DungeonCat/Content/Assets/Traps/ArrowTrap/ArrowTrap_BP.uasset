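; Arrow trap that starts disguised with placeholder materials and hidden doors, and fires arrows at nearby TopDownCharacters.
; An outer overlap drives a timeline that scales doors open and slides the holes.
; After a short delay, inner overlap restores original materials and enables Tick-driven, staggered three-pair arrow volleys on a cooldown.
; Tick also computes Thief-distance visibility while undiscovered, and reveals and closes the trap when inactive.
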(event `self.ReceiveBeginPlay`
  (bind _arrowtrap_main (`self.ArrowTrap_Main`))
  (bind _holes (`self.Holes`))
  ;[1 1 1] Event Begin Play - set positions of arrowstart
  (`|ExecutionSequence`
    (:`then_0`
      (set `self.ArrowPositions_01` (`|MakeArray` (`self.ArrowPos_01`) (`self.ArrowPos_02`)))
      (set `self.ArrowPositions_02` (`|MakeArray` (`self.ArrowPos_03`) (`self.ArrowPos_04`)))
      (set `self.ArrowPositions_03` (`|MakeArray` (`self.ArrowPos_05`) (`self.ArrowPos_06`))))
    (:`then_1`
      ;[1 1 1] Set Transp Mat
      (set `self.OrgMaterials_Holes` (`MeshComponent.GetMaterials` (`self.Holes`)))
      (set `self.OrgMaterials` (`MeshComponent.GetMaterials` (`self.ArrowTrap_Main`)))
      (`|ExecutionSequence`
        (:`then_0`
          (`PrimitiveComponent.SetMaterial` _arrowtrap_main 0 "/Game/Assets/WorldMaterials/TrapMaterials/Trap_StoneGrey.Trap_StoneGrey")
          (`PrimitiveComponent.SetMaterial` _arrowtrap_main 1 "/Game/Assets/WorldMaterials/TrapMaterials/Trap_StoneGrey.Trap_StoneGrey")
          (`PrimitiveComponent.SetMaterial` _arrowtrap_main 2 "/Game/Assets/WorldMaterials/TrapMaterials/Trap_StoneGrey.Trap_StoneGrey")
          (`PrimitiveComponent.SetMaterial` _arrowtrap_main 3 "/Game/Assets/WorldMaterials/TrapMaterials/Trap_Red.Trap_Red"))
        (:`then_1`
          (`PrimitiveComponent.SetMaterial` _holes 1 "/Game/Assets/WorldMaterials/TrapMaterials/Trap_Red.Trap_Red")
          (`PrimitiveComponent.SetMaterial` _holes 0 "/Game/Assets/WorldMaterials/TrapMaterials/Trap_Red.Trap_Red"))
        (:`then_2`
          (`SceneComponent.SetVisibility` (`self.Door_01`) false false)
          (`SceneComponent.SetVisibility` (`self.Door_02`) false false))))))

(event `Event Tick #2`
  ;[1 1 1] SET TRANSP MAT - Sjukt Ooptimerat, fixa
  (if (`self.IsActive?`)
    (if (not (`self.IsFound?`))
      (if (`self.IsActiveThief?`)
        (set `self.Visbility` (`KismetMathLibrary.FClamp` (- (+ (* (`KismetMathLibrary.MapRangeClamped` (/ (`KismetMathLibrary.VSize` (- (`self.K2_GetActorLocation` (`self.Thief`)) (`self.K2_GetActorLocation` self))) 10.0) 10.0 100.0 0.0 1.0) -1.0) 1.0) (`self.VisbilityMinus`))))))
    (else
      (`/Engine/EditorBlueprintResources/StandardMacros.DoOnce` false
        (:`Completed`
          (`self.Reset Materials`)
          (`self.ReverseTimeline`))))))

(event `self.ArrowTrapOuterDetect.OnComponentBeginOverlap`
  (params (OtherActor :type "Actor Object Reference") (OtherComp :type "PrimitiveComponent Object Reference") (OtherBodyIndex :type Integer) (bFromSweep :type Boolean) (SweepResult :type "HitResult Structure (by ref)"))
  ;[1 1 1] Open Doors on proximity
  (if (`self.IsActive?`)
    (cast `/Game/Blueprints/Blueprints/TopDownCharacter` OtherActor)
    (`|ExecutionSequence`
      (:`then_0`
        (bind (_direction _newtrack_0) (`Timeline|Timeline_0` :!via `PlayFromStart` :!label _label)
          (:`Update`
            (`|ExecutionSequence`
              (:`then_0`
                (`SceneComponent.SetRelativeScale3D` (`self.Door_01`) (`KismetMathLibrary.VLerp` (1.0 1.0 1.0) (1.0 0.0 1.0) _newtrack_0))
                (`SceneComponent.SetRelativeScale3D` (`self.Door_02`) (`KismetMathLibrary.VLerp` (1.0 1.0 1.0) (1.0 0.0 1.0) _newtrack_0)))
              (:`then_1`
                (`SceneComponent.K2_SetRelativeLocation` (`self.Holes`) (`KismetMathLibrary.VLerp` (0.0 0.0 0.0) (-3.3 0.0 0.0) _newtrack_0) false false)))))))))

(event `ReverseTimeline`
  ;[1 1 1] Open Doors on proximity
  (goto _label :!via `Reverse`))

(event `self.ArrowTrapOuterDetect.OnComponentEndOverlap`
  (params (OtherActor :type "Actor Object Reference") (OtherComp :type "PrimitiveComponent Object Reference") (OtherBodyIndex :type Integer))
  ;[1 1 1] Open Doors on proximity
  (if (`self.IsActive?`)
    (cast `/Game/Blueprints/Blueprints/TopDownCharacter` OtherActor)
    (`|ExecutionSequence`
      (:`then_0`
        (goto _label :!via `ReverseFromEnd`)))))

(event `self.ArrowTrapInnerDetect.OnComponentBeginOverlap`
  (params (OtherActor :type "Actor Object Reference") (OtherComp :type "PrimitiveComponent Object Reference") (OtherBodyIndex :type Integer) (bFromSweep :type Boolean) (SweepResult :type "HitResult Structure (by ref)"))
  ;[1 1 1] Start/End Shooting on inner Proximity
  (cast `/Game/Blueprints/Blueprints/TopDownCharacter` OtherActor)
  (`KismetSystemLibrary.Delay` 0.2)
  (set `self.ArrowTrapActivate` true)
  (`/Engine/EditorBlueprintResources/StandardMacros.DoOnce` false
    (:`Completed`
      (set `self.IsFound?` true)
      (`self.Reset Materials`))))

(event `self.ArrowTrapInnerDetect.OnComponentEndOverlap`
  (params (OtherActor :type "Actor Object Reference") (OtherComp :type "PrimitiveComponent Object Reference") (OtherBodyIndex :type Integer))
  ;[1 1 1] Start/End Shooting on inner Proximity
  (cast `/Game/Blueprints/Blueprints/TopDownCharacter` OtherActor)
  (`KismetSystemLibrary.Delay` 0.2)
  (set `self.ArrowTrapActivate` false))

(event `self.ReceiveTick`
  (params (DeltaSeconds :type "Float (single-precision)"))
  ;[1 1 1] FIRE FIRE FIRE!
  (`self.Event Tick #2`)
  (if (`self.IsActive?`)
    (if (`self.ArrowTrapActivate`)
      (`/Engine/EditorBlueprintResources/StandardMacros.DoOnce` false :!label _label_2
        (:`Completed`
          (`|ExecutionSequence`
            (:`then_0`
              (for _array_element (`self.ArrowPositions_01`)
                (`|SpawnActorFromClass` "/Game/Assets/Traps/ArrowTrap/ArrowBP.ArrowBP_C" (`KismetMathLibrary.MakeTransform` (.location (`SceneComponent.K2_GetComponentToWorld` _array_element)) (.rotation (`SceneComponent.K2_GetComponentToWorld` _array_element))) "AdjustIfPossibleButAlwaysSpawn" "OverrideRootScale")))
            (:`then_1`
              (`KismetSystemLibrary.Delay` 0.2)
              (for _array_element_2 (`self.ArrowPositions_02`)
                (`|SpawnActorFromClass` "/Game/Assets/Traps/ArrowTrap/ArrowBP.ArrowBP_C" (`KismetMathLibrary.MakeTransform` (.location (`SceneComponent.K2_GetComponentToWorld` _array_element_2)) (.rotation (`SceneComponent.K2_GetComponentToWorld` _array_element_2))) "AdjustIfPossibleButAlwaysSpawn" "OverrideRootScale")))
            (:`then_2`
              (`KismetSystemLibrary.Delay` 0.4)
              (for _array_element_3 (`self.ArrowPositions_03`)
                (`|SpawnActorFromClass` "/Game/Assets/Traps/ArrowTrap/ArrowBP.ArrowBP_C" (`KismetMathLibrary.MakeTransform` (.location (`SceneComponent.K2_GetComponentToWorld` _array_element_3)) (.rotation (`SceneComponent.K2_GetComponentToWorld` _array_element_3))) "AdjustIfPossibleButAlwaysSpawn" "OverrideRootScale")))
            (:`then_3`
              (`KismetSystemLibrary.Delay` 1.5)
              (goto _label_2 :!via `Reset`))))))))

(fn `Reset Materials`
  (for (_array_element _array_index) (`self.OrgMaterials`)
    (`PrimitiveComponent.SetMaterial` (`self.ArrowTrap_Main`) _array_index _array_element)
    (`PrimitiveComponent.SetMaterial` (`self.Door_02`) _array_index _array_element)
    (`PrimitiveComponent.SetMaterial` (`self.Door_01`) _array_index _array_element)
    (`SceneComponent.SetVisibility` (`self.Door_02`) true false)
    (`SceneComponent.SetVisibility` (`self.Door_01`) true false)
    (for (_array_element_2 _array_index_2) (`self.OrgMaterials_Holes`)
      (`PrimitiveComponent.SetMaterial` (`self.Holes`) _array_index_2 _array_element_2))))

(fn `UserConstructionScript`)