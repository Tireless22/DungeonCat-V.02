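; Arrow projectile for the arrow trap that shows an impact effect when it hits something.
; On spawn, its mesh collision stays off for a brief moment, and the actor destroys itself after a timeout.
; On hit it destroys itself and spawns the ArrowHit emitter at the arrow's position.
; For a TopDownCharacter, the emitter instead attaches near the off-hand item with random jitter, and a debug HIT prints; no damage is applied here.
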(event `self.ReceiveBeginPlay`
  (bind _staticmesh (`self.StaticMesh`))
  (`PrimitiveComponent.SetCollisionEnabled` _staticmesh "NoCollision")
  (`KismetSystemLibrary.Delay` 0.02)
  (`PrimitiveComponent.SetCollisionEnabled` _staticmesh "QueryAndPhysics")
  (`KismetSystemLibrary.Delay` 10.0)
  (`self.K2_DestroyActor`))

(event `self.StaticMesh.OnComponentHit`
  (params (OtherActor :type "Actor Object Reference") (OtherComp :type "PrimitiveComponent Object Reference") (NormalImpulse :type "Vector Structure") (Hit :type "HitResult Structure (by ref)"))
  (set `self.transform` (`SceneComponent.K2_GetComponentToWorld` (`self.StaticMesh`)))
  (`self.K2_DestroyActor`)
  (bind _astop_down_character (cast `/Game/Blueprints/Blueprints/TopDownCharacter` OtherActor)
    (:`then`
      (bind _offhanditemcomponent (`/Game/Blueprints/Blueprints/TopDownCharacter.OffHandItemComponent` _astop_down_character))
      (`GameplayStatics.SpawnEmitterAttached` "/Game/Assets/VFX/ArrowHit.ArrowHit" _offhanditemcomponent "LeftHand_ItemJointSocket" (+ (`SceneComponent.K2_GetComponentLocation` _offhanditemcomponent) (`KismetMathLibrary.MakeVector` (`KismetMathLibrary.Conv_IntToDouble` (`KismetMathLibrary.Round` (`KismetMathLibrary.RandomFloatInRange` -10.0 10.0))) (`KismetMathLibrary.Conv_IntToDouble` (`KismetMathLibrary.Round` (`KismetMathLibrary.RandomFloatInRange` -10.0 10.0))) (`KismetMathLibrary.Conv_IntToDouble` (`KismetMathLibrary.Round` (`KismetMathLibrary.RandomFloatInRange` -7.0 7.0))))) (`SceneComponent.K2_GetComponentRotation` _offhanditemcomponent) "KeepWorldPosition")
      (`KismetSystemLibrary.PrintString` "HIT" true true (struct :`R` 1.0 :`G` 0.03117 :`A` 1.0)))
    (:`CastFailed`
      (`GameplayStatics.SpawnEmitterAtLocation` "/Game/Assets/VFX/ArrowHit.ArrowHit" (.location (`self.transform`)) (.rotation (`self.transform`))))))

(fn `UserConstructionScript`)