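; Moving cliff actor that shuttles back and forth between its starting spot and a point offset along world X.
; BeginPlay caches the mesh's world transform, and two timelines lerp the actor location out and back without sweeping.
; Each timeline's finish flips a direction bool and restarts the other for an endless loop, while Tick keeps calling Play on the timeline matching that bool.
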(event `self.ReceiveBeginPlay`
  (set `self.StartPos` (`SceneComponent.K2_GetComponentToWorld` (`self.StaticMeshComponent`))))

(event `self.ReceiveTick`
  (params (DeltaSeconds :type "Float (single-precision)"))
  (if (`self.NewVar_0`)
    (bind (_direction _newtrack_0) (`Timeline|Timeline_0` :!label _label)
      (:`Update`
        (`self.K2_SetActorLocation` (.location (`KismetMathLibrary.TLerp` (`self.StartPos`) (`KismetMathLibrary.MakeTransform` (+ (.location (`self.StartPos`)) (1000.0 0.0 0.0)) (.rotation (`self.StartPos`)) (.scale (`self.StartPos`))) _newtrack_0))))
      (:`Finished`
        (set `self.NewVar_0` false)
        (bind (_direction_2 _newtrack_0_2) (`Timeline|Timeline_1` :!via `PlayFromStart` :!label _label_2)
          (:`Update`
            (`self.K2_SetActorLocation` (.location (`KismetMathLibrary.TLerp` (`KismetMathLibrary.MakeTransform` (+ (.location (`self.StartPos`)) (1000.0 0.0 0.0)) (.rotation (`self.StartPos`)) (.scale (`self.StartPos`))) (`self.StartPos`) _newtrack_0_2))))
          (:`Finished`
            (set `self.NewVar_0` true)
            (goto _label :!via `PlayFromStart`)))))
    (else
      (goto _label_2))))

(fn `UserConstructionScript`)