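; Chest actor that a TopDownCharacter can pick up and drop with the right trigger, highlighted via custom depth on overlap.
; Tick polls the first overlapping character; pickup disables physics, lerps the mesh to the left-hand socket by timeline and briefly pauses movement.
; Warriors sheathe their weapon and restore its prior state after dropping.
; Dropping re-enables physics and opens a short window pushing the transform through SetServerPosition each tick.
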(event `self.ReceiveTick`
  (params (DeltaSeconds :type "Float (single-precision)"))
  (bind _tempactor (`self.TempActor`))
  (bind _tempactor_2 (`self.TempActor`))
  (bind _chestskeletalmesh (`self.ChestSkeletalMesh`))
  (`|ExecutionSequence`
    (:`then_0`
      (bind _astop_down_character (cast `/Game/Blueprints/TopDownCharacter` (`self.TempActor`)))
      (if (`PrimitiveComponent.IsOverlappingComponent` (`self.InRangeDetect`) (`Character.CapsuleComponent` _astop_down_character))
        (bind _rtrigger_pressed (`/Game/Blueprints/TopDownCharacter.RTrigger_Pressed` _astop_down_character))
        (if _rtrigger_pressed
          (if (not (`self.TriggerVar`))
            (`/Engine/EditorBlueprintResources/StandardMacros.DoOnce` false :!label _label
              (:`Completed`
                (`PrimitiveComponent.SetEnableGravity` _chestskeletalmesh false)
                (`PrimitiveComponent.SetSimulatePhysics` _chestskeletalmesh false)
                (set `self.PhysWindow` false)
                (bind __ (`self.IsWarrior?` (`self.TempActor`))
                  (:`Out`
                    (if __
                      (set `self.WasSheathed?` (`/Game/Blueprints/TopDownCharacter.SheathedWeapon` _astop_down_character)))
                    (`|ExecutionSequence`
                      (:`then_0`
                        ;[1 1 1] ChestInterpolationToJointPos
                        (set `self.TempChestLoc` (`SceneComponent.K2_GetComponentToWorld` (`self.ChestSkeletalMesh`)))
                        (bind (_direction _newtrack_0) (`Timeline|Timeline_0` :!via `PlayFromStart`)
                          (:`Update`
                            (`SceneComponent.K2_SetWorldTransform` (`self.ChestSkeletalMesh`) (`KismetMathLibrary.TLerp` (`self.TempChestLoc`) (`SceneComponent.GetSocketTransform` (`Character.Mesh` _astop_down_character) "LeftHand_ItemJointSocket" "RTS_World") _newtrack_0) false false))))
                      (:`then_1`
                        (bind ___2 (`self.IsWarrior?` _tempactor_2)
                          (:`Out`
                            (if ___2
                              (`self.Warrior Chest Toggles Off` _tempactor_2
                                (:`Out`
                                  _)))
                            (set `/Game/Blueprints/TopDownCharacter.ChestPickUpTrigger` true _astop_down_character)
                            (set `self.ChestIsPickedUp?` true)
                            (bind _charactermovement (`Character.CharacterMovement` _astop_down_character))
                            (`ActorComponent.SetActive` _charactermovement false false)
                            (`KismetSystemLibrary.Delay` 1.16)
                            (`PrimitiveComponent.SetRenderCustomDepth` (`self.ChestSkeletalMesh`) false)
                            (`ActorComponent.SetActive` _charactermovement true false)
                            (set `self.TriggerVar` true)
                            (goto _label_2 :!via `Reset`)))))))))))))
    (:`then_1`
      (if (`self.TriggerVar`)
        (if _rtrigger_pressed
          (`/Engine/EditorBlueprintResources/StandardMacros.DoOnce` true :!label _label_2
            (:`Completed`
              (set `/Game/Blueprints/TopDownCharacter.ChestPickUpTrigger` false _astop_down_character)
              (set `self.ChestIsPickedUp?` false)
              (`PrimitiveComponent.SetEnableGravity` _chestskeletalmesh true)
              (`PrimitiveComponent.SetSimulatePhysics` _chestskeletalmesh true)
              (`|ExecutionSequence`
                (:`then_0`
                  (`KismetSystemLibrary.Delay` 0.6)
                  (set `/Game/Blueprints/TopDownCharacter.ChestLerpDone?` false _astop_down_character)
                  (set `self.TriggerVar` false)
                  (bind ___3 (`self.IsWarrior?` _tempactor)
                    (:`Out`
                      (if ___3
                        (`self.Warrior Chest Toggles On` _tempactor
                          (:`Out`
                            (goto _label :!via `Reset`)))
                        (else
                          (goto _label :!via `Reset`))))))
                (:`then_1`
                  ;[1 1 1] Time When server Updates Physics-Position
                  (set `self.PhysWindow` true)
                  (`KismetSystemLibrary.Delay` 2.0)
                  (set `self.PhysWindow` false))))))))
    (:`then_2`
      (if (`self.PhysWindow`)
        (`self.Update Object`)))))

(event `self.ReceiveActorBeginOverlap`
  (params (OtherActor :type "Actor Object Reference"))
  (cast `/Game/Blueprints/TopDownCharacter` OtherActor)
  (`PrimitiveComponent.SetRenderCustomDepth` (`self.ChestSkeletalMesh`) true)
  (`/Engine/EditorBlueprintResources/StandardMacros.DoOnce` false :!label _label_3
    (:`Completed`
      (set `self.TempActor` OtherActor))))

(event `self.ReceiveActorEndOverlap`
  (params (OtherActor :type "Actor Object Reference"))
  (cast `/Game/Blueprints/TopDownCharacter` OtherActor)
  (`PrimitiveComponent.SetRenderCustomDepth` (`self.ChestSkeletalMesh`) false)
  (if (== OtherActor (`self.TempActor`))
    (goto _label_3 :!via `Reset`)))

(event `Update Object`
  (`self.SetServerPosition` (`SceneComponent.K2_GetComponentToWorld` (`self.ChestSkeletalMesh`))))

(event `SetServerPosition`
  (params (NewParam :type "Transform Structure"))
  (`SceneComponent.K2_SetWorldTransform` (`self.ChestSkeletalMesh`) NewParam false true))

(fn `OnRep_WorldTransform`)

(fn `UserConstructionScript`)