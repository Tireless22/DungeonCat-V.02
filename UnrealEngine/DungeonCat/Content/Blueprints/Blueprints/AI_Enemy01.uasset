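; AI_Enemy01 is an enemy character that wanders the navmesh, chases the player on sight and makes melee attacks.
; Tick issues random roaming moves until PawnSensing spots the player, then AI MoveTo closes in and triggers AttackPlayer.
; The attack halves walk speed, plays an animation and applies delayed damage if still in range.
; A raised shield negates damage when AttackCone's yaw comparison finds the enemy within the player's 100-degree facing cone.
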(event `AttackCone`
  (bind _yaw (.yaw (`SceneComponent.K2_GetComponentRotation` (`self.Mesh`))))
  (bind _yaw_2 (.yaw (`SceneComponent.K2_GetComponentRotation` (`Character.Mesh` (`self.TopDownCharRef`)))))
  (bind _returnvalue (- _yaw_2 50.0))
  (bind _returnvalue_2 (+ _yaw_2 50.0))
  ;[1 1 1] Oskars AI (Radera Allt detta:)
  ;;[1 1 1] Check to see if blocking player is facing AI in a 100 degree cone
  (if (> _returnvalue_2 180.0)
    (set `self.RotationMax` (- _returnvalue_2 360.0))
    (elif (< _returnvalue_2 -180.0)
      (set `self.RotationMax` (+ _returnvalue_2 360.0))
      (else
        (set `self.RotationMax` _returnvalue_2)
        ;;;[1 1 1] Comment
        (if (> _returnvalue 180.0)
          (set `self.RotationMin` (- _returnvalue 360.0))
          (elif (< _returnvalue -180.0)
            (set `self.RotationMin` (+ _returnvalue 360.0))
            (else
              (set `self.RotationMin` _returnvalue)))))))
  (if (> _yaw 0.0)
    (set `self.AIRotation` (- _yaw 180.0))
    (else
      (set `self.AIRotation` (+ _yaw 180.0))))
  (if (`KismetMathLibrary.InRange_FloatFloat` (`self.AIRotation`) (`self.RotationMin`) (`self.RotationMax`))
    (set `self.BlockConeIsBlocking` true)
    (else
      (set `self.BlockConeIsBlocking` false))))

(event `AttackPlayer`
  (bind _charactermovement (`self.CharacterMovement`))
  (bind _topdowncharref (`self.TopDownCharRef`))
  ;[1 1 1] Oskars AI (Radera Allt detta:)
  ;;[1 1 1] Attacking
  (bind _astop_down_character (cast `/Game/Blueprints/Blueprints/TopDownCharacter` (`GameplayStatics.GetPlayerPawn` 0)))
  (set `self.TopDownCharRef` _astop_down_character)
  (if (< (`self.GetDistanceTo` (`self.TopDownCharRef`)) 200.0)
    (set `CharacterMovementComponent.MaxWalkSpeed` (/ (`CharacterMovementComponent.MaxWalkSpeed` _charactermovement) 2.0) _charactermovement)
    (set `self.IsAttacking` true)
    (`SkeletalMeshComponent.PlayAnimation` (`self.Mesh`) "/Game/Characters/MainCharacter/Animations/MainChar_Attack_Combo_01_01.MainChar_Attack_Combo_01_01" false)
    (`KismetSystemLibrary.Delay` 0.2)
    (if (< (`self.GetDistanceTo` (`self.TopDownCharRef`)) 200.0)
      (if (`/Game/Blueprints/Blueprints/TopDownCharacter.ShieldStance` (`self.TopDownCharRef`))
        (`self.AttackCone`)
        (if (not (`self.BlockConeIsBlocking`))
          (set `/Game/Blueprints/Blueprints/TopDownCharacter.HP` (- (`/Game/Blueprints/Blueprints/TopDownCharacter.HP` _topdowncharref) 10) _topdowncharref :!label _label))
        (else
          (goto _label))))
    (set `CharacterMovementComponent.MaxWalkSpeed` (* (`CharacterMovementComponent.MaxWalkSpeed` (`self.CharacterMovement`)) 2.0) (`self.CharacterMovement`))
    (set `self.IsAttacking` false)
    (`/Game/Blueprints/Blueprints/TopDownCharacter.CheckHP` (`self.TopDownCharRef`))))

(event `self.PawnSensing.OnSeePawn`
  (params (Pawn :type "Pawn Object Reference"))
  ;[1 1 1] Oskars AI (Radera Allt detta:)
  ;;[1 1 1] On see Pawn go there and try to attack when close enough
  (if (not (`self.IsAttacking`))
    (set `self.In range` true)
    (bind _astop_down_character (cast `/Game/Blueprints/Blueprints/TopDownCharacter` Pawn))
    (`|AIMoveTo` self (0.0 0.0 0.0) _astop_down_character 100.0
      (:`OnSuccess`
        (`self.AttackPlayer`))
      (:`OnFail`
        (`KismetSystemLibrary.RetriggerableDelay` 0.5)
        (set `self.In range` false)))))

(event `self.ReceiveTick`
  (params (DeltaSeconds :type "Float (single-precision)"))
  ;[1 1 1] Oskars AI (Radera Allt detta:)
  ;;[1 1 1] Ai Move to random point in area
  (if (`self.In range`)
    _
    (elif (not (`self.Moving`))
      (bind _outactors (`GameplayStatics.GetAllActorsOfClass` "/Script/Engine.RecastNavMesh"))
      (`|AIMoveTo` self (`NavigationSystem.GetRandomPointInNavigableRadius` (`self.K2_GetActorLocation` self) 1500.0 (`KismetArrayLibrary.Array_Get` _outactors)) null 100.0
        (:`then`
          (set `self.Moving` true))
        (:`OnSuccess`
          (set `self.Moving` false :!label _label_2))
        (:`OnFail`
          (goto _label_2))))))

(fn `UserConstructionScript`)