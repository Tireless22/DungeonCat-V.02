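; GameState for the main menu that handles login and character-name checks against SaveGame_Server.
; LoginCheck tests username and password independently, sets the player ID from the username's index, and reports to the MainMenuMaster login widget.
; The name events check for duplicates or save the name at MyPlayerID, then resume the CreateCharacter widget.
; Each event creates a fresh save object instead of loading the slot, so it starts from class defaults.
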(event `LoginCheck`
  (params (Username :type Text) (Password :type Text))
  (bind _returnvalue (`GameplayStatics.CreateSaveGameObject` "/Game/Blueprints/Blueprints/MainMenu/SaveGame_Server.SaveGame_Server_C"))
  (bind _assave_game_server (cast `/Game/Blueprints/Blueprints/MainMenu/SaveGame_Server` _returnvalue))
  (bind _usernamearray (`/Game/Blueprints/Blueprints/MainMenu/SaveGame_Server.UsernameArray` _assave_game_server))
  (if (`KismetArrayLibrary.Array_Contains` _usernamearray Username)
    (set `self.GMUsernameIsWrong` false)
    (bind _outactors (`GameplayStatics.GetAllActorsOfClass` "/Game/Blueprints/Blueprints/MainMenu/MainMenuGameMode.MainMenuGameMode_C"))
    (`/Game/Blueprints/Blueprints/MainMenu/MainMenuGameMode.SetIDAccordingToName` _outactors (`KismetArrayLibrary.Array_Find` _usernamearray Username))
    (else
      (set `self.GMUsernameIsWrong` true)))
  (if (`KismetArrayLibrary.Array_Contains` (`/Game/Blueprints/Blueprints/MainMenu/SaveGame_Server.PasswordArray` _assave_game_server) Password)
    (set `self.GMPasswordIsWrong` false)
    (else
      (set `self.GMPasswordIsWrong` true)))
  (bind _foundwidgets (`WidgetBlueprintLibrary.GetAllWidgetsOfClass` "/Game/Blueprints/Widgets/MainMenuMaster.MainMenuMaster_C"))
  (bind _asmain_menu_master (cast `/Game/Blueprints/Widgets/MainMenuMaster` (`KismetArrayLibrary.Array_Get` _foundwidgets))
    (:`then`
      (`/Game/Blueprints/Widgets/MainMenuLogin.ContinueLogin` (`/Game/Blueprints/Widgets/MainMenuMaster.MainMenuLogin` _asmain_menu_master) (`self.GMUsernameIsWrong`) (`self.GMPasswordIsWrong`) false))
    (:`CastFailed`
      (`KismetSystemLibrary.PrintString` "FailCastLoginwrongright"))))

(event `CharacterNameCheck`
  (params (CharacterName :type Text))
  (bind _returnvalue (`GameplayStatics.CreateSaveGameObject` "/Game/Blueprints/Blueprints/MainMenu/SaveGame_Server.SaveGame_Server_C"))
  (bind _assave_game_server (cast `/Game/Blueprints/Blueprints/MainMenu/SaveGame_Server` _returnvalue)
    (:`then`
      (bind _foundwidgets (`WidgetBlueprintLibrary.GetAllWidgetsOfClass` "/Game/Blueprints/Widgets/CreateCharacter.CreateCharacter_C"))
      (bind _ascreate_character (cast `/Game/Blueprints/Widgets/CreateCharacter` (`KismetArrayLibrary.Array_Get` _foundwidgets)))
      (`/Game/Blueprints/Widgets/CreateCharacter.CharacterNameContinue` _ascreate_character (`KismetArrayLibrary.Array_Contains` (`/Game/Blueprints/Blueprints/MainMenu/SaveGame_Server.CharacterName` _assave_game_server) CharacterName)))
    (:`CastFailed`
      (`KismetSystemLibrary.PrintString` "failcast3"))))

(event `CharacterSaveName`
  (params (Name :type Text))
  (bind _returnvalue (`GameplayStatics.CreateSaveGameObject` "/Game/Blueprints/Blueprints/MainMenu/SaveGame_Server.SaveGame_Server_C"))
  (bind _assave_game_server (cast `/Game/Blueprints/Blueprints/MainMenu/SaveGame_Server` _returnvalue))
  (bind _asmain_menu_controller (cast `/Game/Blueprints/Blueprints/MainMenu/MainMenuController` (`GameplayStatics.GetPlayerController` 0))
    (:`then`
      (`KismetArrayLibrary.Array_Set` (`/Game/Blueprints/Blueprints/MainMenu/SaveGame_Server.CharacterName` _assave_game_server) (`/Game/Blueprints/Blueprints/MainMenu/MainMenuController.MyPlayerID` _asmain_menu_controller) Name)
      (`GameplayStatics.SaveGameToSlot` _assave_game_server "SaveGame_Server")
      (bind _foundwidgets (`WidgetBlueprintLibrary.GetAllWidgetsOfClass` "/Game/Blueprints/Widgets/CreateCharacter.CreateCharacter_C"))
      (bind _ascreate_character (cast `/Game/Blueprints/Widgets/CreateCharacter` (`KismetArrayLibrary.Array_Get` _foundwidgets))
        (:`then`
          (`/Game/Blueprints/Widgets/CreateCharacter.ContinueOpenLevel` _ascreate_character))
        (:`CastFailed`
          (`KismetSystemLibrary.PrintString` "failcast5"))))
    (:`CastFailed`
      (`KismetSystemLibrary.PrintString` "failcast4"))))

(fn `UserConstructionScript`)