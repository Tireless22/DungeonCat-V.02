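; Laser ability actor that knocks back characters it overlaps and bursts on impact.
; An overlapped TopDownCharacter, other than the actor's owner, is switched to Falling and launched along the Collision component's forward vector with upward lift, overriding its current velocity.
; A blocking hit spawns the ArrowHit particle effect aligned to the surface normal and destroys the actor.
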(event `self.ReceiveHit`
  (params (MyComp :type "PrimitiveComponent Object Reference") (Other :type "Actor Object Reference") (OtherComp :type "PrimitiveComponent Object Reference") (bSelfMoved :type Boolean) (HitLocation :type "Vector Structure") (HitNormal :type "Vector Structure") (NormalImpulse :type "Vector Structure") (Hit :type "HitResult Structure (by ref)"))
  (`GameplayStatics.SpawnEmitterAtLocation` "/Game/Assets/VFX/ArrowHit.ArrowHit" HitLocation (`KismetMathLibrary.Conv_VectorToRotator` HitNormal))
  (`self.K2_DestroyActor`))

(event `self.ReceiveActorBeginOverlap`
  (params (OtherActor :type "Actor Object Reference"))
  (bind _astop_down_character (cast `/Game/Blueprints/TopDownCharacter` OtherActor))
  (if (not (== (`self.GetOwner`) OtherActor))
    (`CharacterMovementComponent.SetMovementMode` (`Character.CharacterMovement` _astop_down_character) "MOVE_Falling" 0)
    (`Character.LaunchCharacter` _astop_down_character (`KismetMathLibrary.MakeVector` (.x (* (`SceneComponent.GetForwardVector` (`self.collision`)) 800.0)) (.y (* (`SceneComponent.GetForwardVector` (`self.collision`)) 800.0)) 500.0) true true)))

(event `self.ReceiveActorEndOverlap`
  (params (OtherActor :type "Actor Object Reference")))

(fn `UserConstructionScript`)