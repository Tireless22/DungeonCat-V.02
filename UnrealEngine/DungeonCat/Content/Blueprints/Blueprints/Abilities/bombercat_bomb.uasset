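; Bomberman-style bomb actor that explodes after a fuse delay, box-tracing along four axis directions and destroying hit actors up to an effectiveness limit, then itself.
; A per-second countdown re-arms a Tick-driven DoOnce that flashes mesh and light through a delayed-loop macro, ending in a white flash and scale-up.
; Collision switches to blocking once the player character leaves the bomb's overlap.
; Debug prints and persistent trace drawing remain enabled.
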(event `self.ReceiveTick`
  (params (DeltaSeconds :type "Float (single-precision)"))
  (bind _bombmesh (`self.bombmesh`))
  (bind _bombmesh_2 (`self.bombmesh`))
  (bind _pointlight (`self.PointLight`))
  ;[1 1 1] Blinking Red
  (if (`self.DoitAgain`)
    (`/Engine/EditorBlueprintResources/StandardMacros.DoOnce` false :!label _label
      (:`Completed`
        (set `self.DoitAgain` false)
        (if (<= (`self.RemainingFuseTime`) 1.0)
          ;[1 1 1] White Explo
          (`PrimitiveComponent.SetMaterial` _bombmesh 0 "/Game/Assets/WorldMaterials/color_reaction_materials/cr_red.cr_red")
          (`KismetSystemLibrary.Delay` 0.5)
          (`PrimitiveComponent.SetMaterial` _bombmesh 0 "/Game/Assets/WorldMaterials/color_reaction_materials/cr_white.cr_white")
          (bind (_direction _newtrack_0) (`Timeline|Explosion Scale` :!via `PlayFromStart`)
            (:`Update`
              (bind _returnvalue (`KismetMathLibrary.Lerp` 0.6 1.0 _newtrack_0))
              (`SceneComponent.SetRelativeScale3D` (`self.bombmesh`) (`KismetMathLibrary.MakeVector` _returnvalue _returnvalue _returnvalue))))
          (else
            (`self.ForLoopWithDelay` 0 (`self.Index`) (/ (`self.RemainingFuseTime`) (* (`self.FuseTime`) 2.0))
              (:`LoopBody`
                (`PrimitiveComponent.SetMaterial` _bombmesh_2 0 "/Game/Assets/WorldMaterials/color_reaction_materials/cr_red.cr_red")
                (`LightComponent.SetLightColor` _pointlight (struct :`R` 1.0 :`G` 0.48648 :`B` 0.475 :`A` 1.0) true)
                (`KismetSystemLibrary.Delay` (/ (/ (`self.RemainingFuseTime`) (* (`self.FuseTime`) 2.0)) 2.0))
                (`PrimitiveComponent.SetMaterial` _bombmesh_2 0 "/Game/Assets/WorldMaterials/Black01.Black01")
                (`LightComponent.SetLightColor` _pointlight (struct :`R` 1.0 :`G` 1.0 :`B` 1.0 :`A` 1.0) true)))))))
    (else
      (goto _label :!via `Reset`))))

(event `self.ReceiveBeginPlay`
  (bind _fusetime (`self.FuseTime`))
  (bind _bombeffectiveness (`self.BombEffectiveness`))
  (bind _returnvalue (`SceneComponent.K2_GetComponentLocation` (`self.bombmesh`)))
  ;[1 1 1] Timer on spawn
  (`|ExecutionSequence`
    (:`then_0`
      (`KismetSystemLibrary.Delay` _fusetime)
      (`KismetSystemLibrary.PrintString` "BOOM")
      ;[1 1 1] Call Explosion func.
      (`|ExecutionSequence`
        (:`then_0`
          (`self.RayCastAndDestroy` _returnvalue (- _returnvalue (`KismetMathLibrary.MakeVector` (`self.BombRange`))) _bombeffectiveness))
        (:`then_1`
          (`self.RayCastAndDestroy` _returnvalue (- _returnvalue (`KismetMathLibrary.MakeVector` (* -1 (`self.BombRange`)))) _bombeffectiveness))
        (:`then_2`
          (`self.RayCastAndDestroy` _returnvalue (- _returnvalue (`KismetMathLibrary.MakeVector` 0.0 (`self.BombRange`))) _bombeffectiveness))
        (:`then_3`
          (`self.RayCastAndDestroy` _returnvalue (- _returnvalue (`KismetMathLibrary.MakeVector` 0.0 (* -1 (`self.BombRange`)))) _bombeffectiveness))
        (:`then_4`
          (`self.K2_DestroyActor` self))))
    (:`then_1`
      (set `self.RemainingFuseTime` _fusetime)
      (bind _index (`self.ForLoopWithDelay` 0 (`KismetMathLibrary.FTrunc` _fusetime) 1.0)
        (:`LoopBody`
          (bind _output_get (set `self.RemainingFuseTime` (- (`self.RemainingFuseTime`) 1.0)))
          (`KismetSystemLibrary.PrintString` (`KismetStringLibrary.Conv_DoubleToString` _output_get))
          (set `self.Index` _index)
          (set `self.DoitAgain` true))))))

(event `self.ReceiveActorBeginOverlap`
  (params (OtherActor :type "Actor Object Reference")))

(event `self.ReceiveActorEndOverlap`
  (params (OtherActor :type "Actor Object Reference"))
  ;[1 1 1] Let player spawn the bomb without collision
  (cast `/Game/Blueprints/TopDownCharacter` OtherActor)
  (`PrimitiveComponent.SetCollisionResponseToAllChannels` (`self.BoxCollision`) "ECR_Block"))

(fn `NewFunction_0`)

(fn `RayCastAndDestroy`
  (params (Start :type "Vector Structure") (End :type "Vector Structure") (BombEffectiveness :type Integer))
  (bind _outhits (`KismetSystemLibrary.BoxTraceMultiForObjects` :`Start` Start :`End` End :`HalfSize` (25.0 25.0 25.0) :`Orientation` (struct) :`ObjectTypes` (`|MakeArray` "ObjectTypeQuery3" "ObjectTypeQuery1" "ObjectTypeQuery2" :!type "EObjectTypeQuery Enum") :`DrawDebugType` "Persistent"))
  (for (_array_element _array_index) _outhits
    (if (<= _array_index BombEffectiveness)
      (`self.K2_DestroyActor` (`.HitActor` (`GameplayStatics.BreakHitResult` _array_element)))
      (else
        (return))))
  (return))

(fn `UserConstructionScript`)