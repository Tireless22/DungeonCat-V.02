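; Rocket ability actor that knocks overlapping TopDownCharacters into the air.
; On overlap it sets the character to Falling and launches it along the collision component's forward direction with a fixed upward boost, overriding existing velocity.
; A Gate opened after a short delay from BeginPlay keeps early overlaps from launching the owner, while other characters are launched immediately.
; The Hit handler has no effect.
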(event `self.ReceiveHit`
  (params (MyComp :type "PrimitiveComponent Object Reference") (Other :type "Actor Object Reference") (OtherComp :type "PrimitiveComponent Object Reference") (bSelfMoved :type Boolean) (HitLocation :type "Vector Structure") (HitNormal :type "Vector Structure") (NormalImpulse :type "Vector Structure") (Hit :type "HitResult Structure (by ref)"))
  (if (!= Other "/Game/Blueprints/TopDownCharacter.TopDownCharacter")
    _))

(event `self.ReceiveBeginPlay`
  (`KismetSystemLibrary.Delay` 1.5)
  (goto _label :!via `Open`))

(event `self.ReceiveActorBeginOverlap`
  (params (OtherActor :type "Actor Object Reference"))
  (bind _astop_down_character (cast `/Game/Blueprints/TopDownCharacter` OtherActor))
  (if (== (`self.GetOwner`) OtherActor)
    (`/Engine/EditorBlueprintResources/StandardMacros.Gate` true :!label _label
      (:`Exit`
        _)))
  (`CharacterMovementComponent.SetMovementMode` (`Character.CharacterMovement` _astop_down_character) "MOVE_Falling" 0)
  (`Character.LaunchCharacter` _astop_down_character (`KismetMathLibrary.MakeVector` (.x (* (`SceneComponent.GetForwardVector` (`self.collision`)) 800.0)) (.y (* (`SceneComponent.GetForwardVector` (`self.collision`)) 800.0)) 500.0) true true))

(event `self.ReceiveActorEndOverlap`
  (params (OtherActor :type "Actor Object Reference")))

(fn `UserConstructionScript`)