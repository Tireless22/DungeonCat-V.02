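; CharacterText is a main menu text actor that orients itself once relative to the player's camera.
; Two seconds after BeginPlay, it casts the player pawn to MainMenuPawn and sets its rotation so its X axis follows the direction from the camera to its TextRender component.
; If the cast fails, it prints a debug string and keeps its rotation.
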(event `self.ReceiveBeginPlay`
  (`KismetSystemLibrary.Delay` 2.0)
  (bind _asmain_menu_pawn (cast `/Game/Blueprints/Blueprints/MainMenu/MainMenuPawn` (`GameplayStatics.GetPlayerPawn` 0))
    (:`then`
      (`self.SetActorRotation` (`KismetMathLibrary.MakeRotFromX` (- (`SceneComponent.K2_GetComponentLocation` (`self.TextRender`)) (`SceneComponent.K2_GetComponentLocation` (`/Game/Blueprints/Blueprints/MainMenu/MainMenuPawn.Camera` _asmain_menu_pawn))))))
    (:`CastFailed`
      (`KismetSystemLibrary.PrintString` "failcamera"))))

(fn `UserConstructionScript`)