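; SaveGame_Server is a server-side save data Blueprint, by its name, that holds per-player account and character data in parallel arrays indexed by PlayerID.
; MainMenuInfo returns a player's username, password and character name.
; CharacterBodyInfo returns the same player's hair, eye and skin colors.
; Both are read-only lookups with no bounds checks, and their calls in the EventGraph never run.
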(fn `CharacterBodyInfo`
  (params (PlayerID :type Integer))
  (returns (CharacterBodyInfoArray :type "Array of Integer"))
  (return (`|MakeArray` (`KismetArrayLibrary.Array_Get` (`self.HairColor`) PlayerID) (`KismetArrayLibrary.Array_Get` (`self.EyeColor`) PlayerID) (`KismetArrayLibrary.Array_Get` (`self.SkinColor`) PlayerID))))

(fn `MainMenuInfo`
  (params (PlayerID :type Integer))
  (returns (MainMenuInfo :type "Array of Text"))
  (return (`|MakeArray` (`KismetArrayLibrary.Array_Get` (`self.UsernameArray`) PlayerID) (`KismetArrayLibrary.Array_Get` (`self.PasswordArray`) PlayerID) (`KismetArrayLibrary.Array_Get` (`self.CharacterName`) PlayerID))))