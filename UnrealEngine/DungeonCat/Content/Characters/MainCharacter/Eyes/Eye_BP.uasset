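; Eye Blueprint for the main character that plays an endless automatic blink on a fixed interval from BeginPlay.
; One timeline squashes EyeBase's Z scale to zero, then the eye is briefly hidden before a second timeline scales it back open.
; Short delays toggle EyeClosed visibility around the squash, and the opening timeline's finish loops back to the wait.
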(event `self.ReceiveBeginPlay`
  (`|ExecutionSequence`
    (:`then_0`
      ;[1 1 1] Blink
      (`/Engine/EditorBlueprintResources/StandardMacros.DoOnce` false
        (:`Completed`
          (`KismetSystemLibrary.Delay` 4.0 :!label _label)
          (`|ExecutionSequence`
            (:`then_0`
              (bind (_direction _newtrack_0) (`Timeline|Timeline_0` :!via `PlayFromStart`)
                (:`Update`
                  (`SceneComponent.SetRelativeScale3D` (`self.EyeBase`) (`KismetMathLibrary.VLerp` (1.0 1.0 1.0) (1.0 1.0 0.0) _newtrack_0)))
                (:`Finished`
                  (`SceneComponent.SetVisibility` (`self.EyeBase`) false true)
                  (`KismetSystemLibrary.Delay` 0.1)
                  (`SceneComponent.SetVisibility` (`self.EyeBase`) true true)
                  (`|ExecutionSequence`
                    (:`then_0`
                      (bind (_direction_2 _newtrack_2) (`Timeline|Open Eyes` :!via `PlayFromStart`)
                        (:`Update`
                          (`|ExecutionSequence`
                            (:`then_0`
                              (`SceneComponent.SetRelativeScale3D` (`self.EyeBase`) (`KismetMathLibrary.VLerp` (1.0 1.0 0.0) (1.0 1.0 1.0) _newtrack_2)))))
                        (:`Finished`
                          (goto _label))))
                    (:`then_1`
                      (`KismetSystemLibrary.Delay` 0.1)
                      (`SceneComponent.SetVisibility` (`self.EyeClosed`) false false))))))
            (:`then_1`
              (`KismetSystemLibrary.Delay` 0.08)
              (`SceneComponent.SetVisibility` (`self.EyeClosed`) true false))))))))

(event `self.ReceiveTick`
  (params (DeltaSeconds :type "Float (single-precision)")))

(fn `UserConstructionScript`)