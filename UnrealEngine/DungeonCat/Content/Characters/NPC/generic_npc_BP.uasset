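; Generic NPC character that randomizes its look on BeginPlay from hard-coded pools of head meshes and clothing, hair and skin materials.
; SetMeshes picks a head piece, and its OnRep either snaps it to a head socket or slaves it to the body's pose, depending on index.
; HairColorVar actually holds a skin-pool material, shared by a body slot and Head.
; Material picks use inclusive Max=Length, so can index past the array end.
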(event `SetMeshes`
  (bind (_mesh_01 _mesh_02 _mesh_03) (break `/Game/Characters/NPC/NPC_meshes` (make `/Game/Characters/NPC/NPC_meshes` "/Game/Assets/Equipment/Head/Admirals_Hair/Admirals_Hair.Admirals_Hair" "/Game/Assets/Equipment/Head/Hair_01/Hair01.Hair01" "/Game/Assets/Equipment/Head/Hood_01/Hood_01.Hood_01")))
  (set `self.HeadIndex` (`KismetMathLibrary.RandomIntegerInRange` 0 3))
  (set `self.SetHeadMesh` (`KismetArrayLibrary.Array_Get` (`|MakeArray` _mesh_01 _mesh_02 _mesh_03 _mesh_02) (`self.HeadIndex`))))

(event `self.ReceiveBeginPlay`
  (bind _skeletalmeshcomponent (`self.SkeletalMeshComponent`))
  (bind _haircolor (`self.HairColor`))
  (bind _skincolor (`self.SkinColor`))
  (bind _clothingcolor (`self.ClothingColor`))
  (bind _haircolorvar (`self.HairColorVar`))
  (bind (_mat_01 _mat_02 _mat_03 _mat_04 _mat_05 _mat_06 _mat_07 _mat_08 _mat_09) (break `/Game/Characters/NPC/NPC_materials` (make `/Game/Characters/NPC/NPC_materials` "/Game/Assets/WorldMaterials/Black01.Black01" "/Game/Assets/WorldMaterials/Brown01.Brown01" "/Game/Assets/WorldMaterials/Brown_02.Brown_02" "/Game/Assets/WorldMaterials/Brown_03.Brown_03" null "/Game/Assets/WorldMaterials/BoneWhite01.BoneWhite01" "/Game/Assets/WorldMaterials/LightBrown01.LightBrown01" "/Game/Assets/WorldMaterials/Skin01.Skin01" "/Game/Assets/WorldMaterials/SkinLight.SkinLight")))
  (bind (_mat_01_2 _mat_02_2 _mat_03_2 _mat_04_2 _mat_05_2 _mat_06_2 _mat_07_2 _mat_08_2 _mat_09_2) (break `/Game/Characters/NPC/NPC_materials` (make `/Game/Characters/NPC/NPC_materials` "/Game/Assets/WorldMaterials/Grey02.Grey02" "/Game/Assets/WorldMaterials/Blue01.Blue01" "/Game/Assets/WorldMaterials/Brown01.Brown01" "/Game/Assets/WorldMaterials/Red01.Red01" "/Game/Assets/WorldMaterials/Blue02.Blue02" "/Game/Assets/WorldMaterials/Brown_02.Brown_02" "/Game/Assets/WorldMaterials/Green02.Green02" "/Game/Assets/WorldMaterials/Orange.Orange" "/Game/Assets/WorldMaterials/LightBrown01.LightBrown01")))
  (bind (_mat_01_3 _mat_02_3 _mat_03_3 _mat_04_3 _mat_05_3 _mat_06_3 _mat_07_3 _mat_08_3 _mat_09_3) (break `/Game/Characters/NPC/NPC_materials` (make `/Game/Characters/NPC/NPC_materials` "/Game/Assets/WorldMaterials/Black01.Black01" "/Game/Assets/WorldMaterials/Yellow01.Yellow01" "/Game/Assets/WorldMaterials/Brown01.Brown01" "/Game/Assets/WorldMaterials/Red01.Red01" "/Game/Assets/WorldMaterials/Grey01.Grey01" "/Game/Assets/WorldMaterials/Brown_02.Brown_02" "/Game/Assets/WorldMaterials/Pink01.Pink01" "/Game/Assets/WorldMaterials/Orange.Orange" "/Game/Assets/WorldMaterials/LightBrown01.LightBrown01")))
  (bind _item (`KismetArrayLibrary.Array_Get` _clothingcolor (`KismetMathLibrary.RandomIntegerInRange` 0 (`KismetArrayLibrary.Array_Length` _clothingcolor))))
  (set `self.ClothingColor` (`|MakeArray` _mat_01_2 _mat_02_2 _mat_03_2 _mat_04_2 _mat_05_2 _mat_06_2 _mat_07_2 _mat_08_2 _mat_09_2 :!type "MaterialInterface Object Reference"))
  (set `self.HairColor` (`|MakeArray` _mat_01_3 _mat_02_3 _mat_03_3 _mat_04_3 _mat_05_3 _mat_06_3 _mat_07_3 _mat_08_3 _mat_09_3 :!type "MaterialInterface Object Reference"))
  (set `self.SkinColor` (`|MakeArray` _mat_01 _mat_02 _mat_03 _mat_04 _mat_06 _mat_07 _mat_08 _mat_09 :!type "MaterialInterface Object Reference"))
  (`self.SetMeshes`)
  (`PrimitiveComponent.SetMaterial` _skeletalmeshcomponent 2 _item)
  (`PrimitiveComponent.SetMaterial` _skeletalmeshcomponent 3 _item)
  (`PrimitiveComponent.SetMaterial` _skeletalmeshcomponent 4 (`KismetArrayLibrary.Array_Get` _haircolor (`KismetMathLibrary.RandomIntegerInRange` 0 (`KismetArrayLibrary.Array_Length` _haircolor))))
  (set `self.HairColorVar` (`KismetArrayLibrary.Array_Get` _skincolor (`KismetMathLibrary.RandomIntegerInRange` 0 (`KismetArrayLibrary.Array_Length` _skincolor))))
  (`PrimitiveComponent.SetMaterial` _skeletalmeshcomponent 1 _haircolorvar)
  (`PrimitiveComponent.SetMaterial` (`self.Head`) 0 _haircolorvar))

(fn `OnRep_SetHead`
  (bind _headindex (`self.HeadIndex`))
  (`SkinnedMeshComponent.SetSkinnedAssetAndUpdate` (`self.Head`) (`self.SetHeadMesh`))
  (if (or (== _headindex 1) (== _headindex 3))
    (`SceneComponent.K2_AttachTo` (`self.Head`) (`self.SkeletalMeshComponent`) (`.Head_17_7D4F679343A1BD5E7C6A0CB0682ADA35` (break `/Game/Blueprints/Inventory/EquipmentSockets` (make `/Game/Blueprints/Inventory/EquipmentSockets` "Earring_Socket"))) "SnapToTarget" false)
    (else
      (`SkinnedMeshComponent.SetLeaderPoseComponent` (`self.Head`) (`self.SkeletalMeshComponent`)))))

(fn `UserConstructionScript`)