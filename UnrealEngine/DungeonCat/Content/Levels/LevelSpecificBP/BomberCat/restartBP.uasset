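; Trigger area in the BomberCat level where players gather to vote for a rematch or to leave, depending on a mode setting.
; Overlaps flag each top-down character as ready, updating a count text and tagged marker materials.
; When all players are ready, a reversed timeline shows a countdown, cancelled if a ready player steps out.
; On completion it resets characters' skills, then restarts the level on authority; exit mode only prints a message.
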(event `Set Marker Color`
  ;[1 1 1] Set materials on nr of players ready
  (if (== (`self.NrOfReadyActors`) (`self.NrOfPlayers`))
    (set `self.MarkerMaterial` "/Game/Assets/WorldMaterials/color_reaction_materials/cr_green2.cr_green2")
    (elif (> (`self.NrOfReadyActors`) 0)
      (set `self.MarkerMaterial` "/Game/Assets/WorldMaterials/color_reaction_materials/cr_yellow.cr_yellow")
      (else
        (set `self.MarkerMaterial` "/Game/Assets/WorldMaterials/White01.White01"))))
  (for _array_element (`self.GetComponentsByTag` "/Script/Engine.StaticMeshComponent" "RematchAreaMarker")
    (`PrimitiveComponent.SetMaterial` _array_element 0 (`self.MarkerMaterial`))))

(event `self.ReceiveTick`
  (params (DeltaSeconds :type "Float (single-precision)"))
  ;[1 1 1] Debug
)

(event `Update Text`
  (bind _players_ready (`self.Players Ready`))
  ;[1 1 1] Set Text on nr of ready players
  (`SceneComponent.SetVisibility` _players_ready true false)
  (`TextRenderComponent.K2_SetText` _players_ready (`|FormatText` "{Ready Players} / {Total Players} ready {leaveorrematch?}" (`KismetTextLibrary.Conv_IntToText` (`self.NrOfReadyActors`)) (`KismetTextLibrary.Conv_IntToText` (`self.NrOfPlayers`)) (`self.actionType`))))

(event `Server check EndOverlap`
  ;[1 1 1] Logic on Enter/Exit TriggerBox
  (bind _astop_down_character (cast `/Game/Blueprints/TopDownCharacter` (stale `self.ReceiveActorEndOverlap` OtherActor)))
  (if (`/Game/Blueprints/TopDownCharacter.ReadyForRestart` _astop_down_character)
    (set `/Game/Blueprints/TopDownCharacter.ReadyForRestart` false _astop_down_character)
    (if (<= (`self.NrOfReadyActors`) 0)
      (set `self.NrOfReadyActors` 0)
      (else
        (set `self.NrOfReadyActors` (- (`self.NrOfReadyActors`) 1))))
    (`self.Stop Timer`)
    (`self.Update Text`)
    (`self.Set Marker Color`)))

(event `self.ReceiveActorEndOverlap`
  (params (OtherActor :type "Actor Object Reference"))
  ;[1 1 1] Logic on Enter/Exit TriggerBox
  (`self.Server check EndOverlap`))

(event `Server check BeginOverlap`
  ;[1 1 1] Logic on Enter/Exit TriggerBox
  (bind _astop_down_character (cast `/Game/Blueprints/TopDownCharacter` (stale `self.ReceiveActorBeginOverlap` OtherActor)))
  (if (not (`/Game/Blueprints/TopDownCharacter.ReadyForRestart` _astop_down_character))
    (set `/Game/Blueprints/TopDownCharacter.ReadyForRestart` true _astop_down_character)
    (set `self.NrOfReadyActors` (+ (`self.NrOfReadyActors`) 1))
    (`self.Update Text`)
    (`self.Set Marker Color`)
    (if (>= (`self.NrOfReadyActors`) (`self.NrOfPlayers`))
      (`self.Run Timer `))))

(event `self.ReceiveActorBeginOverlap`
  (params (OtherActor :type "Actor Object Reference"))
  ;[1 1 1] Logic on Enter/Exit TriggerBox
  (`self.Server check BeginOverlap`))

(event `Stop Timer`
  (bind (_direction _newtrack_0) (`Timeline|Counter timeline` :!via `Stop` :!label _label)
    (:`Update`
      ;[1 1 1] 5 sec Countdown
      (set `self.Counter` _newtrack_0)
      (`TextRenderComponent.K2_SetText` (`self.Players Ready`) (`|FormatText` "{Event} in {Time left} Seconds" (`self.EventText`) (`KismetTextLibrary.Conv_DoubleToText` (`self.Counter`) "HalfToEven" true 1 3 1 1))))
    (:`Finished`
      (`self.Server Do Important Stuff`))))

(event `Run Timer`
  (goto _label :!via `ReverseFromEnd`))

(event `self.ReceiveBeginPlay`
  (bind _maintext (`self.MainText`))
  ;[1 1 1] Need more stable way of finding all Actors. What if one leaves?
  (bind _outactors (`GameplayStatics.GetAllActorsOfClass` "/Game/Blueprints/TopDownCharacter.TopDownCharacter_C"))
  (set `self.AllCharacterArray` _outactors)
  (`SceneComponent.SetVisibility` (`self.SpriteComponent`) false false)
  ;[1 1 1] Set Text depending on LevelAction
  (switch `int` (`self.RematchBP or ExitBP?`)
    (:`0`
      (set `self.actionType` "for rematch!")
      (`TextRenderComponent.K2_SetText` _maintext (`KismetTextLibrary.Conv_StringToText` "Rematch Area"))
      (set `self.EventText` "Rematch"))
    (:`1`
      (set `self.actionType` "to leave!")
      (`TextRenderComponent.K2_SetText` _maintext (`KismetTextLibrary.Conv_StringToText` "Exit Area"))
      (set `self.EventText` "Leaving"))))

(event `Server Do Important Stuff`
  (for _array_element (`self.AllCharacterArray`)
    (`/Game/Blueprints/TopDownCharacter.BomberCat Reset Skills` _array_element)
    (set `self.NrOfReadyActors` 0)
    (switch `int` (`self.RematchBP or ExitBP?`)
      (:`0`
        ;[1 1 1] REOPEN LEVEL?
        (if (`self.HasAuthority`)
          (`KismetSystemLibrary.PrintString` "RE-Re-Re-REEEEEMAAAAATCH!" true true (struct :`G` 0.66 :`B` 1.0 :`A` 1.0) 5.0)
          (`KismetSystemLibrary.ExecuteConsoleCommand` "RestartLevel")))
      (:`1`
        ;[1 1 1] EXIT LEVEL?
        (`KismetSystemLibrary.PrintString` "R-R-R-RAAAAGGEQUIT" true true (struct :`G` 0.66 :`B` 1.0 :`A` 1.0) 5.0)))))

(fn `UserConstructionScript`)